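; Crossing trigger for a Pac-Man-style mode that changes the direction of a BP_Hunter entering its box.
; On BeginPlay, four line traces against WorldStatic remove blocked directions from the open list.
; On overlap it drops the hunter's retreat direction, then after a short delay sets CurrentDirection from RandomAvailableDirection.
; That function's random array pick appears unconnected, and a debug print loop never runs.
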(event `self.ReceiveBeginPlay`
  ;[1 1 1] On Start: Find Open and Blocked Locations
  (`self.FindOpenAndBlockedDirections`))

(event `self.Box.OnComponentBeginOverlap`
  (params (OverlappedComponent :type "PrimitiveComponent Object Reference") (OtherActor :type "Actor Object Reference") (OtherComp :type "PrimitiveComponent Object Reference") (OtherBodyIndex :type Integer) (bFromSweep :type Boolean) (SweepResult :type "HitResult Structure (by ref)"))
  ;[1 1 1] When Hunter Overlaps: Remove Retreat Option from OpenDirections and give him a new random direction
  (bind _asbp_hunter (cast `/Game/Macht_Helden/Blueprints/Character/BP_Hunter` OtherActor))
  (`self.RemoveRetreatOption` (`/Game/Macht_Helden/Blueprints/Character/BP_Hunter.CurrentDirection` _asbp_hunter))
  (`KismetSystemLibrary.Delay` 0.15)
  (set `/Game/Macht_Helden/Blueprints/Character/BP_Hunter.CurrentDirection` (`self.RandomAvailableDirection`) _asbp_hunter))

(fn `FindOpenAndBlockedDirections`
  (returns (OpenDirections :type "Array of /Game/Macht_Helden/Blueprints/E_Direction Enum") (BlockedDirections :type "Array of /Game/Macht_Helden/Blueprints/E_Direction Enum"))
  (bind _returnvalue (`self.K2_GetActorLocation`))
  (bind _blockeddirections (`self.BlockedDirections`))
  (bind _opendirections (`self.OpenDirections`))
  (bind _blockeddirections_2 (`self.BlockedDirections`))
  ;[1 1 1] Check for blocking objects in 4 Directions.
  (for _index (range 4)
    (bind (_outhit _returnvalue_2) (`KismetSystemLibrary.LineTraceSingleForObjects` :`Start` _returnvalue :`End` (+ _returnvalue (* (select `bool` (< _index 2) :`false` (`self.GetActorRightVector`) :`true` (`self.GetActorForwardVector`)) (select `int` _index :`0` 150.0 :`1` -150.0 :`2` -150.0 :`3` 150.0 :!type "Float (single-precision)"))) :`ObjectTypes` (`|MakeArray` "ObjectTypeQuery1" :!type "EObjectTypeQuery Enum") :`DrawDebugType` "ForDuration"))
    ;[1 1 1] If Linetrace finds a blocking object, Add to BlockedDirections Array
    (if _returnvalue_2
      (switch `int` _index
        (:`0`
          (`KismetArrayLibrary.Array_AddUnique` _blockeddirections_2 "NewEnumerator0"))
        (:`1`
          (`KismetArrayLibrary.Array_AddUnique` _blockeddirections_2 "NewEnumerator1"))
        (:`2`
          (`KismetArrayLibrary.Array_AddUnique` _blockeddirections_2 "NewEnumerator2"))
        (:`3`
          (`KismetArrayLibrary.Array_AddUnique` _blockeddirections_2 "NewEnumerator3")))))
  ;[1 1 1] When completed Remove Blocked Directions from Open Directions
  (for _array_element _blockeddirections
    (`KismetArrayLibrary.Array_RemoveItem` _opendirections _array_element))
  (return _opendirections _blockeddirections))

(fn `RemoveRetreatOption`
  (params (Index :type "/Game/Macht_Helden/Blueprints/E_Direction Enum" :default "NewEnumerator0"))
  (bind _output (`|GetArrayItem` (`self.DirectionSelector`) (select `/Game/Macht_Helden/Blueprints/E_Direction` Index :`NewEnumerator0` 1 :`NewEnumerator2` 3 :`NewEnumerator3` 2)))
  ;[1 1 1] Reset Available Directions. Get Retreat Direction based on Current Direction and remove it as option for further movement
  (bind _output_get (set `self.AvailableDirections` (`self.OpenDirections`)))
  (if (`KismetArrayLibrary.Array_Contains` _output_get _output)
    (`KismetArrayLibrary.Array_RemoveItem` _output_get _output))
  (return))

(fn `UserConstructionScript`)