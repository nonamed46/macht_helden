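; BP_Ghost is a player-controllable character that moves continuously in its current direction and keeps a score.
; Up, Down, Left and Right inputs call events that set CurrentDirection, which Tick turns into signed movement input along vectors from CalcMovementDirection.
; UpdateScore adds a change, clamps the score at zero and prints it.
; The construction script applies WalkSpeed to the movement component.
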(event `self.ReceiveTick`
  (params (DeltaSeconds :type "Float (single-precision)"))
  (bind (_returnvalue _returnvalue2) (`self.CalcMovementDirection`))
  (bind _currentdirection (`self.CurrentDirection`))
  (bind _returnvalue_2 (select `/Game/Macht_Helden/Blueprints/E_Direction` _currentdirection :`NewEnumerator0` 1.0 :`NewEnumerator1` -1.0 :`NewEnumerator2` -1.0 :`NewEnumerator3` 1.0 :!type "Float (single-precision)"))
  ;[1 1 1] On Tick: Movement
  (switch `/Game/Macht_Helden/Blueprints/E_Direction` _currentdirection
    (:`NewEnumerator0`
      (`self.AddMovementInput` _returnvalue _returnvalue_2 :!label _label))
    (:`NewEnumerator1`
      (goto _label))
    (:`NewEnumerator2`
      (`self.AddMovementInput` _returnvalue2 _returnvalue_2 :!label _label_2))
    (:`NewEnumerator3`
      (goto _label_2))))

(event `InputAction|Up`
  (params (Key :type "Key Structure"))
  ;[1 1 1] Manual Direction Change
  (:`Pressed`
    (`self.MoveUp`)))

(event `MoveUp`
  ;[1 1 1] Manual Direction Change
  (set `self.CurrentDirection` "NewEnumerator0"))

(event `MoveDown`
  ;[1 1 1] Manual Direction Change
  (set `self.CurrentDirection` "NewEnumerator1"))

(event `InputAction|Down`
  (params (Key :type "Key Structure"))
  ;[1 1 1] Manual Direction Change
  (:`Pressed`
    (`self.MoveDown`)))

(event `MoveLeft`
  ;[1 1 1] Manual Direction Change
  (set `self.CurrentDirection` "NewEnumerator2"))

(event `InputAction|Left`
  (params (Key :type "Key Structure"))
  ;[1 1 1] Manual Direction Change
  (:`Pressed`
    (`self.MoveLeft`)))

(event `MoveRight`
  ;[1 1 1] Manual Direction Change
  (set `self.CurrentDirection` "NewEnumerator3"))

(event `InputAction|Right`
  (params (Key :type "Key Structure"))
  ;[1 1 1] Manual Direction Change
  (:`Pressed`
    (`self.MoveRight`)))

(event `UpdateScore`
  (params (ScoreChange :type "Float (double-precision)"))
  (bind _output_get (set `self.Score` (`KismetMathLibrary.FMax` (+ ScoreChange (`self.Score`)))))
  (`KismetSystemLibrary.PrintString` (`KismetStringLibrary.Conv_DoubleToString` _output_get) true true (struct :`G` 0.66 :`B` 1.0 :`A` 1.0) 4.0))

(fn `UserConstructionScript`
  (set `CharacterMovementComponent.MaxWalkSpeed` (`self.WalkSpeed`) (`self.CharacterMovement`)))