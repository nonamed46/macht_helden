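; BP_PacGhost is a Pac-Man-style ghost character that wanders in four directions at a configurable walk speed.
; Each Tick adds signed movement input for CurrentDirection along axes from CalcMovementDirection, whose control-yaw vector nodes appear unconnected.
; UpdateDirection randomly keeps the current direction or turns 90 degrees, never reversing; nothing in this Blueprint calls it.
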(event `self.ReceiveTick`
  (params (DeltaSeconds :type "Float (single-precision)"))
  (bind (_returnvalue _returnvalue2) (`self.CalcMovementDirection`))
  (bind _currentdirection (`self.CurrentDirection`))
  (bind _returnvalue_2 (select `/Game/Macht_Helden/Blueprints/E_Direction` _currentdirection :`NewEnumerator0` 1.0 :`NewEnumerator1` -1.0 :`NewEnumerator2` -1.0 :`NewEnumerator3` 1.0 :!type "Float (single-precision)"))
  ;[1 1 1] On Tick: Movement
  (switch `/Game/Macht_Helden/Blueprints/E_Direction` _currentdirection
    (:`NewEnumerator0`
      (`self.AddMovementInput` _returnvalue _returnvalue_2 :!label _label))
    (:`NewEnumerator1`
      (goto _label))
    (:`NewEnumerator2`
      (`self.AddMovementInput` _returnvalue2 _returnvalue_2 :!label _label_2))
    (:`NewEnumerator3`
      (goto _label_2))))

(event `UpdateDirection`
  (bind _returnvalue (`KismetMathLibrary.RandomIntegerInRange` 0 2))
  ;[1 1 1] Change Direction based on Current Direction. Never use 180° turns!
  (switch `/Game/Macht_Helden/Blueprints/E_Direction` (`self.CurrentDirection`)
    (:`NewEnumerator0`
      (switch `int` _returnvalue ; O: Up
        (:`0`
          (set `self.CurrentDirection` "NewEnumerator0" :!label _label_3))
        (:`1`
          (set `self.CurrentDirection` "NewEnumerator2" :!label _label_4))
        (:`2`
          (set `self.CurrentDirection` "NewEnumerator3" :!label _label_5))))
    (:`NewEnumerator1`
      (switch `int` _returnvalue ; O: Down
        (:`0`
          (set `self.CurrentDirection` "NewEnumerator1" :!label _label_6))
        (:`1`
          (goto _label_4))
        (:`2`
          (goto _label_5))))
    (:`NewEnumerator2`
      (switch `int` _returnvalue ; O: Left
        (:`0`
          (goto _label_3))
        (:`1`
          (goto _label_6))
        (:`2`
          (goto _label_4))))
    (:`NewEnumerator3`
      (switch `int` _returnvalue ; O: Right
        (:`0`
          (goto _label_3))
        (:`1`
          (goto _label_6))
        (:`2`
          (goto _label_5))))))

(fn `UserConstructionScript`
  (set `CharacterMovementComponent.MaxWalkSpeed` (`self.WalkSpeed`) (`self.CharacterMovement`)))