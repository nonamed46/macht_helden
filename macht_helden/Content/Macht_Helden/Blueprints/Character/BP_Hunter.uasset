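; BP_Hunter is a character Blueprint that moves continuously along one of four directions held in CurrentDirection.
; Tick feeds AddMovementInput one of two CalcMovementDirection vectors, one per axis, with the sign selected by direction.
; CalcMovementDirection contains yaw-only control-rotation forward and right vector nodes, shown as unconnected.
; The construction script copies WalkSpeed into the movement component's MaxWalkSpeed.
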(event `self.ReceiveTick`
  (params (DeltaSeconds :type "Float (single-precision)"))
  (bind (_returnvalue _returnvalue2) (`self.CalcMovementDirection`))
  (bind _currentdirection (`self.CurrentDirection`))
  (bind _returnvalue_2 (select `/Game/Macht_Helden/Blueprints/E_Direction` _currentdirection :`NewEnumerator0` 1.0 :`NewEnumerator1` -1.0 :`NewEnumerator2` -1.0 :`NewEnumerator3` 1.0 :!type "Float (single-precision)"))
  ;[1 1 1] On Tick: Movement
  (switch `/Game/Macht_Helden/Blueprints/E_Direction` _currentdirection
    (:`NewEnumerator0`
      (`self.AddMovementInput` _returnvalue _returnvalue_2 :!label _label))
    (:`NewEnumerator1`
      (goto _label))
    (:`NewEnumerator2`
      (`self.AddMovementInput` _returnvalue2 _returnvalue_2 :!label _label_2))
    (:`NewEnumerator3`
      (goto _label_2))))

(fn `UserConstructionScript`
  (set `CharacterMovementComponent.MaxWalkSpeed` (`self.WalkSpeed`) (`self.CharacterMovement`)))